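; BP_Potion is a carryable potion that shrinks or grows the player character.
; Pickup snaps it to the passed skeletal mesh's right-hand socket and disables its collision.
; Primary and secondary use each run a FlipFlop, finding BP_ThirdPersonCharacterCustom by class and toggling it between small or giant and normal scale.
; Drop detaches the potion, restores collision and simulates physics briefly before switching simulation off.
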(event EventBeginPlay)

(event Collision|EventActorBeginOverlap
  (params (OtherActor :type Actor%20Object%20Reference)))

(event EventTick
  (params (DeltaSeconds :type Float%20%28single-precision%29)))

(event EventPickup
  (params (Skeletal%20Mesh :type Skeletal%20Mesh%20Component%20Object%20Reference))
  ;[0.15 0.15 0.15 0.5] Picks Up Potion
  (Development|PrintString "You picked up a potion")
  (Transformation|AttachComponentToComponent Skeletal%20Mesh "hand_r" "SnapToTarget" "SnapToTarget" "SnapToTarget" true)
  (Collision|SetCollisionEnabled (Variables|Default|GetPotion) "NoCollision"))

(event EventUsePrimary
  ;[0.15 0.15 0.15 0.5] Shrinks (Left Key)
  (Utilities|FlowControl|FlipFlop
    (:A
      (Development|PrintText "You Shrank!")
      (bind _returnvalue (Actor|GetActorOfClass "/Game/Blueprints/Evelyn_Blueprints/BP_ThirdPersonCharacterCustom.BP_ThirdPersonCharacterCustom_C"))
      (Transformation|SetActorScale3D _returnvalue "0.200000,0.200000,0.200000"))
    (:B
      (Transformation|SetActorScale3D _returnvalue "1.000000,1.000000,1.000000"))))

(event EventDrop
  (bind _potion (Variables|Default|GetPotion))
  ;[0.15 0.15 0.15 0.5] Drop Potion
  (Transformation|DetachFromActor "KeepWorld" "KeepWorld" "KeepWorld")
  (Physics|SetSimulatePhysics _potion true)
  (Collision|SetCollisionEnabled _potion "QueryAndPhysics")
  (Utilities|FlowControl|Delay 2.0)
  (Physics|SetSimulatePhysics (Variables|Default|GetPotion) false))

(event EventUseSecondary
  ;[0.15 0.15 0.15 0.5] Grow
  (Utilities|FlowControl|FlipFlop
    (:A
      (Development|PrintText "My how much you've grown!")
      (bind _returnvalue (Actor|GetActorOfClass "/Game/Blueprints/Evelyn_Blueprints/BP_ThirdPersonCharacterCustom.BP_ThirdPersonCharacterCustom_C"))
      (Transformation|SetActorScale3D _returnvalue "3.000000,3.000000,3.000000"))
    (:B
      (Transformation|SetActorScale3D _returnvalue "1.000000,1.000000,1.000000"))))

(fn ConstructionScript)