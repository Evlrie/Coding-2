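; Base enemy AI controller that runs BT_EnemyBase on possession and seeds its blackboard with the pawn's attack and strafe ranges.
; AI Perception updates route successful sight, hearing, damage and prediction stimuli to handlers that set the blackboard state, target or point of interest.
; Seeing the player or taking damage triggers Attacking; hearing the player or any prediction triggers Investigating.
; Failed stimuli only print, so the sight-loss prediction request is never reached.
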(event OnTargetPerceptionUpdated(AIPerception)
  (params (Actor :type Actor%20Object%20Reference) (Stimulus :type AI%20Stimulus%20Structure))
  (bind (_age _expirationage _strength _stimuluslocation _receiverlocation _tag _bsuccessfullysensed) (Utilities|Struct|BreakAIStimulus Stimulus))
  (bind _returnvalue (Class|AIPerceptionSystem|GetSenseClassforStimulus Stimulus))
  (if _bsuccessfullysensed
    (switch string (Utilities|GetClassDisplayName _returnvalue)
      (:AISense_Sight
        (Development|PrintText "SIGHT" true true "(R=0.539931,G=0.403665,B=0.090440,A=1.000000)")
        (CallFunction|OnSeeTarget Actor _bsuccessfullysensed _stimuluslocation))
      (:AISense_Hearing
        (Development|PrintText "HEARING")
        (CallFunction|OnHearTarget Actor _stimuluslocation _bsuccessfullysensed))
      (:AISense_Damage
        (Development|PrintText "DAMAGE")
        (CallFunction|OnRecieveDamage Actor))
      (:AISense_Prediction
        (Development|PrintText "PREDICTION")
        (CallFunction|OnPredictTarget _stimuluslocation)))
    (else
      (Development|PrintText "Not Sensed"))))

(event EventBeginPlay)

(event EventTick
  (params (DeltaSeconds :type Float%20%28single-precision%29)))

(event EventPossess
  (params (PossessedPawn :type Pawn%20Object%20Reference))
  (bind _asbp_enemy_base (Utilities|Casting|CastToBP_EnemyBase PossessedPawn))
  (Variables|Default|SetAs%20BP%20Enemy%20Base _asbp_enemy_base)
  (AI|RunBehaviorTree "/Game/Blueprints/AI_Enemy/BT_EnemyBase.BT_EnemyBase")
  (CallFunction|SetState "NewEnumerator0" (Game|GetPlayerCharacter 0))
  (AI|Components|Blackboard|SetValueasFloat (Variables|Default|GetBlackboard) (Utilities|Name|MakeLiteralName "AttackRadius") (.AttackRadius (Default|GetIdealRange (Variables|Default|GetAs%20BP%20Enemy%20Base))))
  (AI|Components|Blackboard|SetValueasFloat (Variables|Default|GetBlackboard) (Utilities|Name|MakeLiteralName "StrafefRadius") (.StrafeRadius (Default|GetIdealRange (Variables|Default|GetAs%20BP%20Enemy%20Base))))
  (Development|PrintText (Utilities|Text|FormatText "attackR: {atkR}: {strfR}" (.AttackRadius (Default|GetIdealRange (Variables|Default|GetAs%20BP%20Enemy%20Base))) (.StrafeRadius (Default|GetIdealRange (Variables|Default|GetAs%20BP%20Enemy%20Base))))))

(fn ConstructionScript)

(fn SetState
  (params (NewState :type E_AIState%20Enum :default "NewEnumerator0") (Attack%20Target :type Actor%20Object%20Reference))
  (AI|Components|Blackboard|SetValueasEnum (Variables|Default|GetBlackboard) (Utilities|Name|MakeLiteralName "State") NewState)
  (if (Utilities|Select :Index NewState :NewEnumerator0 false :NewEnumerator1 false :NewEnumerator2 true :NewEnumerator3 false)
    (AI|Components|Blackboard|SetValueasObject (Variables|Default|GetBlackboard) (Utilities|Name|MakeLiteralName "AttackTarget") Attack%20Target)))

(fn OnSeeTarget
  (params (Target :type Actor%20Object%20Reference) (Sucessfully%20Sensed :type Boolean) (Last%20known%20location :type Vector))
  (if Sucessfully%20Sensed
    (Development|PrintString "I see an Enmemy ")
    (switch Utilities|FlowControl|Switch|SwitchonE_AIState (Utilities|Enum|ByteToEnumE_AIState (Class|BlackboardComponent|GetValueasEnum (Variables|Default|GetBlackboard) (Utilities|Name|MakeLiteralName "State")))
      (:NewEnumerator0
        _)
      (:NewEnumerator1
        _)
      (:NewEnumerator3
        _))
    (Utilities|Casting|CastToBP_ThirdPersonCharacter Target
      (:then
        (CallFunction|SetState "NewEnumerator2" Target))
      (:CastFailed
        (Development|PrintText "That is Not my Enemy")))
    (else
      (Development|PrintString "Lost Sight of Player")
      (switch Utilities|FlowControl|Switch|SwitchonE_AIState (Utilities|Enum|ByteToEnumE_AIState (Class|BlackboardComponent|GetValueasEnum (Variables|Default|GetBlackboard) (Utilities|Name|MakeLiteralName "State")))
        (:NewEnumerator2
          (Utilities|Casting|CastToBP_ThirdPersonCharacter Target)
          (Development|PrintString "Lost Sight of Enemy")
          (Class|AISensePrediction|RequestPawnPredictionEvent (Pawn|GetControlledPawn) Target 1.0))))))

(fn OnHearTarget
  (params (Target :type Actor%20Object%20Reference) (Pont%20of%20Interest :type Vector) (Successfully%20Sensed :type Boolean))
  (if Successfully%20Sensed
    (Development|PrintString "What was that?")
    (switch Utilities|FlowControl|Switch|SwitchonE_AIState (Utilities|Enum|ByteToEnumE_AIState (Class|BlackboardComponent|GetValueasEnum (Variables|Default|GetBlackboard) (Utilities|Name|MakeLiteralName "State")))
      (:NewEnumerator0
        _)
      (:NewEnumerator1
        _)
      (:NewEnumerator3
        _))
    (Utilities|Casting|CastToBP_ThirdPersonCharacter Target)
    (AI|Components|Blackboard|SetValueasVector (Variables|Default|GetBlackboard) (Utilities|Name|MakeLiteralName "Point of Interest") Pont%20of%20Interest)
    (CallFunction|SetState "NewEnumerator3" Target)
    (else
      (Development|PrintString "It must have been nothing"))))

(fn OnRecieveDamage
  (params (Attack%20Target :type Actor%20Object%20Reference))
  (switch Utilities|FlowControl|Switch|SwitchonE_AIState (Utilities|Enum|ByteToEnumE_AIState (Class|BlackboardComponent|GetValueasEnum (Variables|Default|GetBlackboard) (Utilities|Name|MakeLiteralName "State")))
    (:NewEnumerator0
      _)
    (:NewEnumerator1
      _)
    (:NewEnumerator3
      _))
  (CallFunction|SetState "NewEnumerator2" Attack%20Target))

(fn OnPredictTarget
  (params (Point%20of%20Interest :type Vector))
  (AI|Components|Blackboard|SetValueasVector (Variables|Default|GetBlackboard) (Utilities|Name|MakeLiteralName "Point of Interest") Point%20of%20Interest)
  (CallFunction|SetState "NewEnumerator3"))