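; BP_Rocks is a throwable rock actor that can be picked up and tossed.
; Pickup prints a message, snaps the rock to the hand_r socket of the supplied skeletal mesh and disables its collision.
; Drop detaches it, enables physics and collision, and applies an impulse along the camera's forward vector scaled by ThrowStrenght.
; After a short delay, it turns physics and collision off and plays a rock sound at its location.
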(event EventBeginPlay)

(event Collision|EventActorBeginOverlap
  (params (OtherActor :type Actor%20Object%20Reference)))

(event EventTick
  (params (DeltaSeconds :type Float%20%28single-precision%29)))

(event EventPickup
  (params (Skeletal%20Mesh :type Skeletal%20Mesh%20Component%20Object%20Reference))
  ;[0.15 0.15 0.15 0.5] Picks Up Radio
  (Development|PrintString "You picked up a rock")
  (Transformation|AttachComponentToComponent Skeletal%20Mesh "hand_r" "SnapToTarget" "SnapToTarget" "SnapToTarget" true)
  (Collision|SetCollisionEnabled (Variables|Default|GetSphere) "NoCollision"))

(event EventDrop
  ;[0.15 0.15 0.15 0.5] Drops Radio
  (Transformation|DetachFromActor "KeepWorld" "KeepWorld" "KeepWorld")
  (Physics|SetSimulatePhysics (Variables|Default|GetSphere) true)
  (Collision|SetCollisionEnabled (Variables|Default|GetSphere) "QueryAndPhysics")
  (Physics|AddImpulse (Variables|Default|GetSphere) (* (Math|Vector|GetForwardVector (Camera|GetCameraRotation (Game|GetPlayerCameraManager 0))) (Variables|Default|GetThrow%20Strenght)) "None" false)
  (Utilities|FlowControl|Delay 1.0)
  (Physics|SetSimulatePhysics (Variables|Default|GetSphere) false)
  (Collision|SetCollisionEnabled (Variables|Default|GetSphere) "NoCollision")
  (Audio|PlaySoundatLocation "/Game/Blueprints/Sounds/RockAudio_Cue.RockAudio_Cue" (Transformation|GetActorLocation) "0, 0, 0" 1.0 1.0 0.0 0 0 0 0))

(fn ConstructionScript)