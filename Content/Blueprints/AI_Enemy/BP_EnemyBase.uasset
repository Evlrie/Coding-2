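; Base enemy Blueprint that repeatedly moves toward the player controller and offers randomized appearance and a melee attack.
; BeginPlay starts an AIMoveTo loop that retries one second after success or failure.
; Separate events randomize the name text, skeletal mesh and material, though the second material pick overwrites the first on the same slot.
; Attack plays a kick montage, then calls AttackFinished on completion or interruption, without applying damage.
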(event Custom|Change%20Text
  (Rendering|Components|TextRender|SetText (Variables|Default|GetAI%20Name%20Text) (.OutItem (Utilities|Array|Random (Utilities|Array|MakeArray (Utilities|Text|MakeLiteralText "Legolas") (Utilities|Text|MakeLiteralText "Gimli") (Utilities|Text|MakeLiteralText "Aragorn"))))))

(event Custom|Change%20Mesh
  (Components|SkeletalMesh|SetSkeletalMeshAsset (Variables|Character|GetMesh) (.OutItem (Utilities|Array|Random (Utilities|Array|MakeArray "/Game/SCK_Casual01/Models/Premade_Characters/MESH_PC_03.MESH_PC_03" "/Engine/Tutorial/SubEditors/TutorialAssets/Character/TutorialTPP.TutorialTPP" "/Game/Characters/Mannequins/Meshes/SKM_Quinn.SKM_Quinn")))))

(event Custom|Change%20Material
  (bind _mesh (Variables|Character|GetMesh))
  (Rendering|Material|SetMaterial _mesh 0 (.OutItem (Utilities|Array|Random (Utilities|Array|MakeArray "/DatasmithContent/Materials/FBXImporter/VRED/BrushedMetal.BrushedMetal" "/Game/Materials/MI_FlatPink.MI_FlatPink" "/AnimationSharing/AnimSharingGreen.AnimSharingGreen"))))
  (Rendering|Material|SetMaterial _mesh 0 (.OutItem (Utilities|Array|Random (Utilities|Array|MakeArray "/Game/Materials/MI_FlatBlue.MI_FlatBlue" "/Niagara/DefaultAssets/GeometryCache/M_DefaultGeometryCacheMaterial_Red.M_DefaultGeometryCacheMaterial_Red" "/DatasmithContent/Materials/FBXImporter/VRED/BrushedMetal.BrushedMetal")))))

(event Custom|Attack
  (Development|PrintString "Attacking Player")
  (Animation|Montage|PlayMontage (Variables|Character|GetMesh) "/Game/CloseCombatAnimSet/Animations/InPlace/Attacks/NinjaWheelKick_Montage.NinjaWheelKick_Montage"
    (:OnCompleted
      _)
    (:OnInterrupted
      _))
  (Default|CallAttackFinished))

(event EventBeginPlay
  (AI|AIMoveTo self "0, 0, 0" (Game|GetPlayerController 0) 2e+02 false :!label _label
    (:OnSuccess
      _)
    (:OnFail
      _))
  (Utilities|FlowControl|Delay 1.0)
  (goto _label))

(fn ConstructionScript)