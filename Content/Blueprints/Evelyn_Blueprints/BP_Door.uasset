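; BP_Door is a locked door that the player opens by spending a key.
; When a BP_ThirdPersonCharacterCustom overlaps its box collision, it checks the character's KeyCount, deducts one key and sets DoorUnlocked so it cannot be unlocked again.
; The DoorOpening timeline then swings the Door component's relative yaw toward -90 degrees.
; Printed messages report success or a missing key.
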(event OnComponentBeginOverlap(BoxCollision)
  (params (OverlappedComponent :type Primitive%20Component%20Object%20Reference) (OtherActor :type Actor%20Object%20Reference) (OtherComp :type Primitive%20Component%20Object%20Reference) (OtherBodyIndex :type Integer) (bFromSweep :type Boolean) (SweepResult :type Hit%20Result%20Structure%20%28by%20ref%29))
  (bind _asbp_third_person_character_custom (Utilities|Casting|CastToBP_ThirdPersonCharacterCustom OtherActor))
  (if (not (Variables|Default|GetDoorUnlocked)) ; Will not unlock if door already has been opened
    (if (> (Variables|/Game/Blueprints/Evelyn_Blueprints/BP_ThirdPersonCharacterCustom.BP_ThirdPersonCharacterCustom_C|GetKeyCount _asbp_third_person_character_custom) 0)
      (Development|PrintString "Open says me!" true true "(R=0.000000,G=1.000000,B=0.026159,A=1.000000)")
      (Variables|/Game/Blueprints/Evelyn_Blueprints/BP_ThirdPersonCharacterCustom.BP_ThirdPersonCharacterCustom_C|SetKeyCount _asbp_third_person_character_custom (- (Variables|/Game/Blueprints/Evelyn_Blueprints/BP_ThirdPersonCharacterCustom.BP_ThirdPersonCharacterCustom_C|GetKeyCount _asbp_third_person_character_custom) 1))
      (Variables|Default|SetDoorUnlocked true)
      (bind _newtrack_0 (Timeline|Door%20Opening Play)
        (:Update
          (Transformation|SetRelativeRotation (Variables|Default|GetDoor) (Math|Rotator|MakeRotator 0.0 0.0 (* _newtrack_0 -9e+01)) false false)))
      (else
        (Development|PrintString "You shall not pass" true true "(R=1.000000,G=0.044257,B=0.000000,A=1.000000)")))))

(event EventBeginPlay)

(event Collision|EventActorBeginOverlap
  (params (OtherActor :type Actor%20Object%20Reference)))

(event EventTick
  (params (DeltaSeconds :type Float%20%28single-precision%29)))

(fn ConstructionScript)