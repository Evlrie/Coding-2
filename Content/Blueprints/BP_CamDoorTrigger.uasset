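; BP_CamDoorTrigger is a trigger actor that opens its Target door when a BP_ThirdPersonCharacter overlaps Sphere1.
; The overlap adds the door uniquely to the GM_SavLoad game mode's SGLevelState DoorOpened list, then calls OpenDoor with the player as the new view target.
; A separate ReopenDoor event calls OpenDoor on the same Target without passing an actor or recording state.
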(event OnComponentBeginOverlap(Sphere1)
  (params (OverlappedComponent :type Primitive%20Component%20Object%20Reference) (OtherActor :type Actor%20Object%20Reference) (OtherComp :type Primitive%20Component%20Object%20Reference) (OtherBodyIndex :type Integer) (bFromSweep :type Boolean) (SweepResult :type Hit%20Result%20Structure%20%28by%20ref%29))
  (Utilities|Casting|CastToBP_ThirdPersonCharacter OtherActor)
  (bind _asgm_sav_load (Utilities|Casting|CastToGM_SavLoad (Game|GetGameMode)))
  (Utilities|Array|AddUnique (Variables|/Game/Blueprints/Evelyn_Blueprints/SG_LevelState.SG_LevelState_C|GetDoorOpened (Variables|/Game/Blueprints/Evelyn_Blueprints/SavingLoading/GM_SavLoad.GM_SavLoad_C|GetSG_LevelState _asgm_sav_load)) (Variables|Default|GetTarget))
  (Default|OpenDoor (Variables|Default|GetTarget) OtherActor) ; new view target is the player
)

(event Custom|ReopenDoor
  (Default|OpenDoor (Variables|Default|GetTarget)))

(event EventBeginPlay)

(event Collision|EventActorBeginOverlap
  (params (OtherActor :type Actor%20Object%20Reference)))

(event EventTick
  (params (DeltaSeconds :type Float%20%28single-precision%29)))

(fn ConstructionScript)