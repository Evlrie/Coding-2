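; BP_MachineGun is an early machine gun weapon that can be picked up, with placeholder firing.
; Pickup attaches it to the hand_r socket of the supplied skeletal mesh and disables collision on MachineGunBody.
; It also switches that body's physics simulation on, then off after a short delay.
; UsePrimary only prints a firing sound as text, with no shooting logic.
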(event EventBeginPlay)

(event Collision|EventActorBeginOverlap
  (params (OtherActor :type Actor%20Object%20Reference)))

(event EventTick
  (params (DeltaSeconds :type Float%20%28single-precision%29)))

(event EventPickup
  (params (Skeletal%20Mesh :type Skeletal%20Mesh%20Component%20Object%20Reference))
  (Development|PrintText "Machine Gun is Picked up")
  (Transformation|AttachComponentToComponent Skeletal%20Mesh "hand_r" "SnapToTarget" "SnapToTarget" "SnapToTarget" true)
  (Physics|SetSimulatePhysics (Variables|Default|GetMachine%20Gun%20Body) true)
  (Collision|SetCollisionEnabled (Variables|Default|GetMachine%20Gun%20Body) "NoCollision")
  (Utilities|FlowControl|Delay 2.0)
  (Physics|SetSimulatePhysics (Variables|Default|GetMachine%20Gun%20Body) false))

(event EventUsePrimary
  (Development|PrintText "BURRRRRRRRRRRRR"))

(fn ConstructionScript)