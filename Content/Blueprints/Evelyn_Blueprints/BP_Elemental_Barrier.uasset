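; BP_Elemental_Barrier is a barrier actor with an elemental type that kills a player who lacks matching immunity.
; On BeginPlay it prints the type and sets its TextRender label to the element's barrier name.
; When the Cube overlaps the custom third-person character, it compares the type with the character's ElementalImmunity.
; On a mismatch it prints a death message, waits briefly, then quits the game.
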(event OnComponentBeginOverlap(Cube)
  (params (OverlappedComponent :type Primitive%20Component%20Object%20Reference) (OtherActor :type Actor%20Object%20Reference) (OtherComp :type Primitive%20Component%20Object%20Reference) (OtherBodyIndex :type Integer) (bFromSweep :type Boolean) (SweepResult :type Hit%20Result%20Structure%20%28by%20ref%29))
  (bind _asbp_third_person_character_custom (Utilities|Casting|CastToBP_ThirdPersonCharacterCustom OtherActor))
  (if (not (Utilities|Enum|Equal(Enum) (Variables|Default|GetElemental%20Type) (Variables|/Game/Blueprints/Evelyn_Blueprints/BP_ThirdPersonCharacterCustom.BP_ThirdPersonCharacterCustom_C|GetElemental%20Immunity _asbp_third_person_character_custom)))
    (Development|PrintText "You're Dead!" true true "(R=1.000000,G=0.019133,B=0.000000,A=1.000000)")
    (Utilities|FlowControl|Delay 2.0)
    (Game|QuitGame 0 "Quit" false)))

(event EventBeginPlay
  (Development|PrintText (|GenerictoText (Variables|Default|GetElemental%20Type)))
  (switch Utilities|FlowControl|Switch|SwitchonElementalType (Variables|Default|GetElemental%20Type)
    (:NewEnumerator1
      (Rendering|Components|TextRender|SetText (Variables|Default|GetTextRender) (Utilities|Text|MakeLiteralText "Barrier of Fire")))
    (:NewEnumerator2
      (Rendering|Components|TextRender|SetText (Variables|Default|GetTextRender) (Utilities|Text|MakeLiteralText "Barrier of Water")))
    (:NewEnumerator3
      (Rendering|Components|TextRender|SetText (Variables|Default|GetTextRender) (Utilities|Text|MakeLiteralText "Barrier of Earth")))
    (:NewEnumerator4
      (Rendering|Components|TextRender|SetText (Variables|Default|GetTextRender) (Utilities|Text|MakeLiteralText "Barrier of Air")))
    (:NewEnumerator5
      (Rendering|Components|TextRender|SetText (Variables|Default|GetTextRender) (Utilities|Text|MakeLiteralText "Barrier of Poison")))
    (:NewEnumerator6
      (Rendering|Components|TextRender|SetText (Variables|Default|GetTextRender) (Utilities|Text|MakeLiteralText "Barrier of Void")))))

(event Collision|EventActorBeginOverlap
  (params (OtherActor :type Actor%20Object%20Reference)))

(event EventTick
  (params (DeltaSeconds :type Float%20%28single-precision%29)))

(fn ConstructionScript)