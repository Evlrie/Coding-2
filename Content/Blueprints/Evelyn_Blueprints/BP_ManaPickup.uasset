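; BP_ManaPickup is a collectible that restores a quarter of the player's mana when touched.
; Its collision overlap casts to BP_ThirdPersonCharacter, calls the Mana function to add the amount clamped between zero and one, refreshes the character's stats, then destroys itself.
; A ManaPickup function with equivalent logic also exists but is not called in this graph.
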(event OnComponentBeginOverlap(collision)
  (params (OverlappedComponent :type Primitive%20Component%20Object%20Reference) (OtherActor :type Actor%20Object%20Reference) (OtherComp :type Primitive%20Component%20Object%20Reference) (OtherBodyIndex :type Integer) (bFromSweep :type Boolean) (SweepResult :type Hit%20Result%20Structure%20%28by%20ref%29))
  (bind _asbp_third_person_character (Utilities|Casting|CastToBP_ThirdPersonCharacter OtherActor))
  (CallFunction|Mana _asbp_third_person_character _asbp_third_person_character)
  (Default|UpdateStats _asbp_third_person_character)
  (Actor|DestroyActor))

(fn ConstructionScript)

(fn ManaPickup
  (params (self2 :type BP%20Third%20Person%20Character%20Object%20Reference) (self3 :type BP%20Third%20Person%20Character%20Object%20Reference))
  (Variables|/Game/ThirdPerson/Blueprints/BP_ThirdPersonCharacter.BP_ThirdPersonCharacter_C|SetMana self2 (Math|Float|Clamp(Float) (+ (Variables|/Game/ThirdPerson/Blueprints/BP_ThirdPersonCharacter.BP_ThirdPersonCharacter_C|GetMana self3) 0.25))))

(fn Mana
  (params (self2 :type BP%20Third%20Person%20Character%20Object%20Reference) (self3 :type BP%20Third%20Person%20Character%20Object%20Reference))
  (Variables|/Game/ThirdPerson/Blueprints/BP_ThirdPersonCharacter.BP_ThirdPersonCharacter_C|SetMana self3 (Math|Float|Clamp(Float) (+ (Variables|/Game/ThirdPerson/Blueprints/BP_ThirdPersonCharacter.BP_ThirdPersonCharacter_C|GetMana self2) 0.25))))