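; Hand radio actor that can be picked up, used to play jazz saxophone music, and dropped.
; Pickup snaps it to the passed skeletal mesh's right-hand socket and disables sphere collision.
; Primary use spawns the music once as a 2D sound, and secondary use toggles pause on that stored audio.
; Drop detaches it and restores collision, simulating sphere physics briefly before switching it off.
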(event EventBeginPlay)

(event Collision|EventActorBeginOverlap
  (params (OtherActor :type Actor%20Object%20Reference)))

(event EventTick
  (params (DeltaSeconds :type Float%20%28single-precision%29)))

(event EventPickup
  (params (Skeletal%20Mesh :type Skeletal%20Mesh%20Component%20Object%20Reference))
  ;[0.15 0.15 0.15 0.5] Picks Up Radio
  (Development|PrintString "You picked up a hand radio")
  (Transformation|AttachComponentToComponent Skeletal%20Mesh "hand_r" "SnapToTarget" "SnapToTarget" "SnapToTarget" true)
  (Collision|SetCollisionEnabled (Variables|Default|GetSphere) "NoCollision"))

(event EventUsePrimary
  ;[0.15 0.15 0.15 0.5] Turns on Music
  (Development|PrintString "Radio Is On")
  (Utilities|FlowControl|DoOnce false
    (:Completed
      (bind _returnvalue (Audio|SpawnSound2D "/Game/Blueprints/Evelyn_Blueprints/Jazz_Saxaphone.Jazz_Saxaphone" 1.0 1.0 0.0 0))
      (Variables|Default|SetMusic _returnvalue))))

(event EventDrop
  (bind _sphere (Variables|Default|GetSphere))
  ;[0.15 0.15 0.15 0.5] Drops Radio
  (Transformation|DetachFromActor "KeepWorld" "KeepWorld" "KeepWorld")
  (Physics|SetSimulatePhysics _sphere true)
  (Collision|SetCollisionEnabled _sphere "QueryAndPhysics")
  (Utilities|FlowControl|Delay 2.0)
  (Physics|SetSimulatePhysics _sphere false))

(event EventUseSecondary
  (bind _music (Variables|Default|GetMusic))
  ;[0.15 0.15 0.15 0.5] Pauses/Resumes Music
  (Utilities|FlowControl|FlipFlop
    (:A
      (Development|PrintString "Pausing Music")
      (Class|AudioComponent|SetPaused _music true))
    (:B
      (Development|PrintString "Resuming Music")
      (Class|AudioComponent|SetPaused _music false))))

(fn ConstructionScript)