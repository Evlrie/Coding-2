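; Game mode that handles saving and loading of player stats and per-level collected-coin state.
; On BeginPlay it loads both save objects or creates new ones, copying saved Stamina, Health and Mana onto the player character and calling AlreadyCollected on each valid saved coin.
; Player stats use a fixed slot, while level state uses the current level name as its slot.
; Separate save events write each held object to disk and print the result.
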(event Custom|Load%20Player%20Stats
  (bind _returnvalue (SaveGame|DoesSaveGameExist "Player Save"))
  (if _returnvalue
    (bind _returnvalue_2 (SaveGame|LoadGamefromSlot "Player Save"))
    (bind _assg_player_stats (Utilities|Casting|CastToSG_PlayerStats _returnvalue_2))
    (Variables|Default|SetSG_PlayerStats _assg_player_stats)
    (bind _asbp_third_person_character (Utilities|Casting|CastToBP_ThirdPersonCharacter (Game|GetPlayerCharacter 0)))
    (Variables|/Game/ThirdPerson/Blueprints/BP_ThirdPersonCharacter.BP_ThirdPersonCharacter_C|SetStamina _asbp_third_person_character (Variables|/Game/Blueprints/Evelyn_Blueprints/SavingLoading/SG_PlayerStats.SG_PlayerStats_C|GetStamina (Variables|Default|GetSG_PlayerStats)))
    (Variables|/Game/ThirdPerson/Blueprints/BP_ThirdPersonCharacter.BP_ThirdPersonCharacter_C|SetHealth _asbp_third_person_character (Variables|/Game/Blueprints/Evelyn_Blueprints/SavingLoading/SG_PlayerStats.SG_PlayerStats_C|GetHealth (Variables|Default|GetSG_PlayerStats)))
    (Variables|/Game/ThirdPerson/Blueprints/BP_ThirdPersonCharacter.BP_ThirdPersonCharacter_C|SetMana _asbp_third_person_character (Variables|/Game/Blueprints/Evelyn_Blueprints/SavingLoading/SG_PlayerStats.SG_PlayerStats_C|GetMana (Variables|Default|GetSG_PlayerStats)))
    (Development|PrintString "PlayerStats have been loaded" true true "(R=0.472783,G=1.000000,B=0.184276,A=1.000000)")
    (else
      (bind _returnvalue_3 (SaveGame|CreateSaveGameObject "/Game/Blueprints/Evelyn_Blueprints/SavingLoading/SG_PlayerStats.SG_PlayerStats_C"))
      (Variables|Default|SetSG_PlayerStats _returnvalue_3) ; set this variable so that th eplayer can edit these values
    )))

(event Custom|SavePlayerStats
  (bind _returnvalue (SaveGame|SaveGametoSlot (Variables|Default|GetSG_PlayerStats) "Player Save"))
  (if _returnvalue
    (Development|PrintText "PlayerStats Written to File" true true "(R=0.090885,G=0.978353,B=1.000000,A=1.000000)")
    (else
      (Development|PrintText "Player Stats could not be written"))))

(event Custom|SaveLevelState
  (bind _returnvalue (Game|GetCurrentLevelName true))
  (bind _returnvalue_2 (SaveGame|SaveGametoSlot (Variables|Default|GetSG_LevelState) _returnvalue))
  (if _returnvalue_2
    (Development|PrintText "LevelState save to game file")
    (else
      (Development|PrintString "Player stats could not be written to saave game file"))))

(event Custom|Load%20Level%20State
  (bind _returnvalue (Game|GetCurrentLevelName true))
  (bind _returnvalue_2 (SaveGame|DoesSaveGameExist _returnvalue))
  (if _returnvalue_2
    (bind _returnvalue_3 (SaveGame|LoadGamefromSlot _returnvalue))
    (bind _assg_level_state (Utilities|Casting|CastToSG_LevelState _returnvalue_3))
    (bind _output_get (Variables|Default|SetSG_LevelState _assg_level_state))
    (for _array_element (Variables|/Game/Blueprints/Evelyn_Blueprints/SG_LevelState.SG_LevelState_C|GetCollectedCoins _output_get)
      (Utilities|IsValid _array_element ; What if coin isn't in level
        (:Is%20Valid
          (Default|AlreadyCollected _array_element))))
    (Development|PrintText "Coin State Loaded")
    (else
      (bind _returnvalue_4 (SaveGame|CreateSaveGameObject "/Game/Blueprints/Evelyn_Blueprints/SG_LevelState.SG_LevelState_C"))
      (Variables|Default|SetSG_LevelState _returnvalue_4))))

(event EventBeginPlay
  (Development|PrintString "Loading the SavLoad Game Mode" true true "(R=0.619792,G=0.285207,B=0.012802,A=1.000000)" 1e+01)
  (CallFunction|LoadPlayerStats)
  (CallFunction|LoadLevelState))

(event EventTick
  (params (DeltaSeconds :type Float%20%28single-precision%29)))

(fn ConstructionScript)