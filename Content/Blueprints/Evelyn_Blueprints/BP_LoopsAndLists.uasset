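; BP_LoopsAndLists is a practice Blueprint that demonstrates loops and arrays through on-screen debug prints.
; BeginPlay starts DelayLoop, an endless self-calling event that prints its counter, waits on a Delay, then increments it.
; After each delay it calls itself both before and after PrintColors.
; PrintColors shuffles and iterates TextColors, printing each line in a random color from a separate inline array, then a completion message.
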(event Custom|Delay%20loop
  (Development|PrintString (Utilities|String|Append "Starting Delay Loop # " "" (Utilities|String|ToString(Integer) (Variables|Default|GetDelayLoopCounter))) true true "(R=0.295561,G=0.074592,B=1.000000,A=1.000000)")
  (Utilities|FlowControl|Delay 1.0)
  (Math|Integer|IncrementInt (Variables|Default|GetDelayLoopCounter)
    (:%20%20
      (CallFunction|DelayLoop)
      (CallFunction|PrintColors)
      (CallFunction|DelayLoop))))

(event Custom|Print%20Colors
  (bind _text_colors (Variables|Default|GetText%20Colors))
  (Utilities|Array|Shuffle _text_colors)
  (for (_ _array_index) _text_colors
    (Development|PrintString (Utilities|String|Append "Printing color # " (Utilities|String|ToString(Integer) _array_index)) true true (.OutItem (Utilities|Array|Random (Utilities|Array|MakeArray "(R=1.000000,G=0.884504,B=0.012599,A=1.000000)" "(R=1.000000,G=0.200699,B=0.173160,A=1.000000)" "(R=0.207598,G=1.000000,B=0.252270,A=1.000000)" "(R=0.236272,G=0.385767,B=1.000000,A=1.000000)")))))
  (Development|PrintString "We are Done Printing colors" true true "(R=0.000000,G=0.000000,B=0.000000,A=1.000000)"))

(event EventBeginPlay
  (Development|PrintString "Loops and lists is active" true true "(R=1.000000,G=0.102827,B=0.908714,A=1.000000)")
  (CallFunction|DelayLoop))

(event Collision|EventActorBeginOverlap
  (params (OtherActor :type Actor%20Object%20Reference)))

(event EventTick
  (params (DeltaSeconds :type Float%20%28single-precision%29)))

(fn ConstructionScript)