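; BP_EnemySpawner is an actor that populates the level with BP_AiMoveTo enemies once at BeginPlay.
; It loops over every BP_EnemySpawnPoint, spawning an enemy at that point's transform with a 75% chance.
; Each spawn calls ChangeText on all BP_AiMoveTo actors in the level, then gives the new enemy a random skeletal mesh from a small fixed set.
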(event EventBeginPlay
  (Development|PrintString "Enemy Spawner is active" true true "(R=1.000000,G=0.232077,B=0.000000,A=1.000000)")
  (bind _outactors (Actor|GetAllActorsOfClass "/Game/Blueprints/Evelyn_Blueprints/BP_EnemySpawnPoint.BP_EnemySpawnPoint_C"))
  (for _array_element _outactors
    (if (Math|Random|RandomBoolwithWeight 0.75)
      (bind _returnvalue (Game|SpawnActorfromClass "/Game/AI_Blueprints/BP_AiMoveTo.BP_AiMoveTo_C" (Transformation|GetActorTransform _array_element) "Undefined" "MultiplyWithRoot" 0 0))
      (bind _outactors_2 (Actor|GetAllActorsOfClass "/Game/AI_Blueprints/BP_AiMoveTo.BP_AiMoveTo_C"))
      (Default|ChangeText _outactors_2)
      (Components|SkeletalMesh|SetSkeletalMeshAsset (Variables|/Script/Engine.Character|GetMesh _returnvalue) (.OutItem (Utilities|Array|Random (Utilities|Array|MakeArray "/Game/SCK_Casual01/Models/Premade_Characters/MESH_PC_03.MESH_PC_03" "/Game/PolygonStarter/Models/Vehicles/SK_Veh_Plane_Stunt_01.SK_Veh_Plane_Stunt_01" "/Game/Characters/Mannequins/Meshes/SKM_Quinn.SKM_Quinn")))))))

(event Collision|EventActorBeginOverlap
  (params (OtherActor :type Actor%20Object%20Reference)))

(event EventTick
  (params (DeltaSeconds :type Float%20%28single-precision%29)))

(fn ConstructionScript)